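; Seesaw actor that rocks its static mesh back and forth within an angle range.
; Each tick advances the angle by Velocity, then applies it to the transform cached at BeginPlay as an inverted pitch offset and a rotation of the relative location around X.
; The move sweeps, and Velocity changes sign at the range bounds.
; Disconnected nodes hold a debug print and a reversal on initial overlap.
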(event EventBeginPlay
  (Variables|Default|SetBaseTransform (Transformation|GetRelativeTransform (Variables|Default|GetStaticMesh))))

(event Collision|EventActorBeginOverlap
  (params (OtherActor :type Actor%20Object%20Reference)))

(event EventTick
  (params (DeltaSeconds :type Float%20%28single-precision%29))
  (bind _anglerange (Variables|Default|GetAngleRange))
  (bind _basetransform (Variables|Default|GetBaseTransform))
  (Variables|Default|SetAngle (+ (* DeltaSeconds (Variables|Default|GetVelocity)) (Variables|Default|GetAngle)))
  (bind _sweephitresult (Transformation|SetRelativeLocationAndRotation (Variables|Default|GetStaticMesh) (Math|Vector|RotateVectorAroundAxis (.location _basetransform) (* (+ (* DeltaSeconds (Variables|Default|GetVelocity)) (Variables|Default|GetAngle)) 1.0) "1.000000,0.000000, 0") (Math|Rotator|MakeRotator (.roll (.rotation _basetransform)) (+ (* (* (+ (* DeltaSeconds (Variables|Default|GetVelocity)) (Variables|Default|GetAngle)) 1.0) -1.0) (.pitch (.rotation _basetransform)) 0.0) (.yaw (.rotation _basetransform))) true false))
  (if (>= (Variables|Default|GetAngle) (.value (.upperbound _anglerange)))
    (Variables|Default|SetVelocity (* (Math|Float|Absolute(Float) (Variables|Default|GetVelocity)) -1.0))
    (elif (>= (.value (.lowerbound _anglerange)) (Variables|Default|GetAngle))
      (Variables|Default|SetVelocity (Math|Float|Absolute(Float) (Variables|Default|GetVelocity))))))

(fn ConstructionScript)