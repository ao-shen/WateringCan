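; Bucket actor that cannot die and shows its inherited Wetness as a liquid level.
; On BeginPlay it caches the Liquid transform and attaches to a named socket on AttachedActor's static meshes, keeping world transform.
; Wetness changes raise and vertically scale the Liquid in proportion to Wetness, using FilledArrow as the height reference.
; Tick applies a fixed negative wetness change every frame, independent of delta time.
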(event EventBeginPlay
  (bind _attachedactor (Variables|Default|GetAttachedActor))
  (bind _liquid (Variables|Default|GetLiquid))
  (bind _socketname (Variables|Default|GetSocketName))
  (bind _returnvalue (Transformation|GetRelativeTransform _liquid))
  (|CallParentFunction)
  (Variables|Default|SetCanDie false)
  (Variables|Default|SetLiquidOffset (.location _returnvalue))
  (Variables|Default|SetLiquidSize (.scale _returnvalue))
  (Utilities|IsValid _attachedactor
    (:Is%20Valid
      (bind _array_element (Utilities|Array|ForEachLoopwithBreak (Actor|GetComponentsByClass _attachedactor "/Script/Engine.StaticMeshComponent") :!label _label)
        (:LoopBody
          (bind _array_element_2 (Utilities|Array|ForEachLoopwithBreak (Transformation|GetAllSocketNames _array_element))
            (:LoopBody
              (if (Utilities|Name|Equal(Name) _array_element_2 _socketname)
                (Transformation|AttachComponentToComponent _array_element _socketname "KeepWorld" "KeepWorld" "KeepWorld" true)
                (goto _label Break)))))))))

(event Collision|EventActorBeginOverlap
  (params (OtherActor :type Actor%20Object%20Reference))
  (|CallParentFunction OtherActor) ; This node is disabled and will not be called.\nDrag off pins to build functionality.
)

(event EventTick
  (params (DeltaSeconds :type Float%20%28single-precision%29))
  (|CallParentFunction DeltaSeconds)
  (CallFunction|ChangeWetness -0.25))

(event EventChangeWetness
  (params (Delta :type Float%20%28single-precision%29))
  (bind _wetness (Variables|Default|GetWetness))
  (bind _liquidsize (Variables|Default|GetLiquidSize))
  (bind _liquidoffset (Variables|Default|GetLiquidOffset))
  (bind _filledarrow (Variables|Default|GetFilledArrow))
  (bind _liquid (Variables|Default|GetLiquid))
  (bind _relativelocation (Variables|/Script/Engine.SceneComponent|GetRelativeLocation _filledarrow))
  (bind _returnvalue (- (.z _relativelocation) (.z _liquidoffset)))
  (bind _returnvalue_2 (* _returnvalue 0.005))
  (bind _returnvalue_3 (* _wetness _returnvalue_2))
  (|CallParentFunction Delta)
  (Transformation|SetRelativeLocation _liquid (+ (Math|Vector|MakeVector 0.0 0.0 _returnvalue_3) (Variables|Default|GetLiquidOffset)) true false)
  (Transformation|SetRelativeScale3D _liquid (Math|Vector|MakeVector (.x _liquidsize) (.y _liquidsize) (* _returnvalue_3 1.0 0.02))))

(fn ConstructionScript
  (|CallParentFunction))