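; Sponge actor that soaks up or loses liquid, tracking it as a wetness percentage.
; ChangeWetness scales the incoming delta by MaxLiquid, feeds CalculateWetness, then maps Wetness to the cube's mass override when the mesh is movable.
; Wetness also drives the GlowColor hue on a dynamic material created in the construction script.
; When IsDead and CanDie are both true, it spawns a water explosion and destroys itself.
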(event Custom|ChangeWetness
  (params (Delta :type Float%20%28single-precision%29))
  (bind _maxmass (Variables|Default|GetMaxMass))
  (bind _cubemesh (Variables|Default|GetCubeMesh))
  (bind _cubemesh_2 (Variables|Default|GetCubeMesh))
  (bind _returnvalue (Transformation|GetWorldTransform _cubemesh_2))
  (Class|BasePhysicsActor|CalculateWetness (* Delta (/ 1e+02 (Variables|Default|GetMaxLiquid))))
  (if (Utilities|Enum|Equal(Enum) (Variables|/Script/Engine.SceneComponent|GetMobility _cubemesh) "Movable")
    (Class|PrimitiveComponent|SetMassOverrideinKg _cubemesh "None" (Math|Float|MapRangeClamped (Variables|Default|GetWetness) 0.0 1e+02 (.value (.lowerbound _maxmass)) (.value (.upperbound _maxmass))) true))
  (Rendering|Material|SetVectorParameterValue (Variables|Default|GetSpongeDynaMat) "GlowColor" (Class|KismetMathLibrary|HSVtoRGB (Math|Float|MapRangeClamped (Variables|Default|GetWetness) 0.0 1e+02 5e+01 2.2e+02) 1.0 1.0 1.0) :!class /Script/Engine.MaterialInstanceDynamic)
  (if (and (Variables|Default|GetisDead) (Variables|Default|GetCanDie))
    (Effects|SpawnEmitteratLocation "/Game/Assets/Particles/WaterExplosion.WaterExplosion" (.location _returnvalue) (.rotation _returnvalue))
    (Actor|DestroyActor)))

(event EventBeginPlay)

(event Collision|EventActorBeginOverlap
  (params (OtherActor :type Actor%20Object%20Reference)))

(event EventTick
  (params (DeltaSeconds :type Float%20%28single-precision%29)))

(fn ConstructionScript
  (bind _returnvalue (Rendering|Material|CreateDynamicMaterialInstance (Variables|Default|GetCubeMesh) 0 0 :!class /Script/Engine.PrimitiveComponent))
  (Variables|Default|SetSpongeDynaMat _returnvalue))