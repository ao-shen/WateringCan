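; Character Blueprint for Fluum that moves at a variable speed and plays a shooting animation when an enemy is found.
; Tick sets max walk speed every frame from SpeedRate times SpeedVariable.
; EnemyFound_Event guards with IsShooting, plays the shoot animation directly on the mesh for a fixed delay, then restores Animation Blueprint mode, with debug prints.
; EnemyLost_Event is an empty stub.
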(event Custom|EnemyFound_Event
  (bind _mesh (Variables|Character|GetMesh))
  (if (not (Variables|Default|GetIsShooting))
    (Development|PrintString "start")
    (Variables|Default|SetIsShooting true)
    (Components|Animation|PlayAnimation _mesh "/Game/AnimationAssets/Fluum/Fluum_Anim_Armature_Shoot.Fluum_Anim_Armature_Shoot" false)
    (Utilities|FlowControl|Delay 2.0)
    (Variables|Default|SetIsShooting false)
    (Components|Animation|SetAnimationMode _mesh "AnimationBlueprint")
    (Development|PrintString "Finish")))

(event Custom|EnemyLost_Event)

(event EventBeginPlay
  (|CallParentFunction) ; This node is disabled and will not be called.\nDrag off pins to build functionality.
)

(event Collision|EventActorBeginOverlap
  (params (OtherActor :type Actor%20Object%20Reference))
  (|CallParentFunction OtherActor) ; This node is disabled and will not be called.\nDrag off pins to build functionality.
)

(event EventTick
  (params (DeltaSeconds :type Float%20%28single-precision%29))
  (|CallParentFunction DeltaSeconds)
  (Variables|/Script/Engine.CharacterMovementComponent|SetMaxWalkSpeed (Variables|Character|GetCharacterMovement) (* (Variables|Default|GetSpeedRate) (Variables|Default|GetSpeedVariable))))

(fn ConstructionScript
  (|CallParentFunction))