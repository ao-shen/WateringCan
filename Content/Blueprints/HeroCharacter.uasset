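; Player character for a twin-stick shooter that spawns a weapon on its gun socket and moves along world axes.
; Each tick, the first touch's offset from screen center sets control yaw to aim.
; Touch press fires until release, while a quick second press throws a grenade with upward velocity set by touch distance.
; On death, it stops firing, then after a delay respawns through TwinStickMode and destroys itself and its weapon.
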(event EventBeginPlay
  (bind _mesh (Variables|Character|GetMesh))
  (Utilities|FlowControl|Sequence
    (:then_0
      (bind _returnvalue (Game|SpawnActorfromClass "/Game/Blueprints/Weapon.Weapon_C" (Transformation|GetWorldTransform _mesh) "AdjustIfPossibleButDontSpawnIfColliding" 0 0))
      (bind _output_get (Variables|Default|SetWeapon _returnvalue))
      (Transformation|AttachComponentToComponent _output_get _mesh "GunSocket" "SnapToTarget" "SnapToTarget" "SnapToTarget" true))
    (:then_1
      (bind _astwin_stick_mode (Utilities|Casting|CastToTwinStickMode (Game|GetGameMode)))
      (bind _output_get_2 (Variables|Default|SetGameMode _astwin_stick_mode))
      (Variables|/Game/Blueprints/TwinStickMode.TwinStickMode_C|SetPlayerSpawnTransform _output_get_2 (Transformation|GetActorTransform)))))

(event Collision|EventActorBeginOverlap
  (params (OtherActor :type Actor%20Object%20Reference)))

(event EventTick
  (params (DeltaSeconds :type Float%20%28single-precision%29))
  (bind _returnvalue (Pawn|GetController))
  ;[1 1 1] Rotation
  (bind _asplayer_controller (Utilities|Casting|CastToPlayerController _returnvalue))
  (if (.bIsCurrentlyPressed (Class|PlayerController|GetInputTouchState _asplayer_controller "Touch1"))
    (bind (_x2 _y2 _distance) (CallFunction|RelativetoCenter (.LocationX (Class|PlayerController|GetInputTouchState _asplayer_controller "Touch1")) (.LocationY (Class|PlayerController|GetInputTouchState _asplayer_controller "Touch1")) _asplayer_controller))
    (Variables|Default|SetDistanceToTouch _distance)
    (Pawn|SetControlRotation _returnvalue (Math|Rotator|MakeRotator (.roll (Math|Conversions|RotationFromXVector (Math|Vector|MakeVector _x2 _y2 0.0))) (.pitch (Math|Conversions|RotationFromXVector (Math|Vector|MakeVector _x2 _y2 0.0))) (+ (.yaw (Math|Conversions|RotationFromXVector (Math|Vector|MakeVector _x2 _y2 0.0))) 9e+01)))))

(event EventAffectHealth
  (params (Delta :type Float%20%28single-precision%29))
  (Class|BaseCharacter|CalculateHealth Delta)
  (Development|PrintString (Utilities|String|ToString(Float) (Variables|Default|GetHealth)))
  (if (Variables|Default|GetisDead)
    (Input|DisableInput 0)
    (Default|ReleaseTrigger (Variables|Default|GetWeapon))
    (Utilities|FlowControl|Delay 3.0)
    (Default|RespawnPlayer (Variables|Default|GetGameMode))
    (Actor|DestroyActor (Variables|Default|GetWeapon))))

(event Input|ActionEvents|InputActionTouchDown
  (params (Key :type Key%20Structure))
  (bind _returnvalue (Actor|GetGameTimeSinceCreation))
  (bind _guntmp (Variables|Default|GetGunTmp))
  (bind _weapon (Variables|Default|GetWeapon))
  (bind _returnvalue_2 (Transformation|GetWorldTransform _guntmp))
  (bind _returnvalue_3 (Math|Vector|RotateVector (Math|Vector|MakeVector 5e+02 0.0 0.0) (.rotation _returnvalue_2)))
  (:Pressed
    (if (< (- _returnvalue (Variables|Default|GetTimeLastTouchDown)) 0.3)
      (Variables|Default|SetTimeLastTouchDown _returnvalue)
      (bind _returnvalue_4 (Game|SpawnActorfromClass "/Game/Blueprints/GrenadeProjectile.GrenadeProjectile_C" (Math|Transform|MakeTransform (.location _returnvalue_2) "0, 0, 0" (.scale _returnvalue_2)) "Undefined" 0 0.0 0))
      (Game|Components|ProjectileMovement|SetVelocityinLocalSpace (Variables|/Game/Blueprints/GrenadeProjectile.GrenadeProjectile_C|GetProjectileMovement _returnvalue_4) (+ (Variables|/Script/Engine.MovementComponent|GetVelocity (Variables|Character|GetCharacterMovement)) (Math|Vector|MakeVector (.x _returnvalue_3) (.y _returnvalue_3) (Variables|Default|GetDistanceToTouch))))
      (else
        (Variables|Default|SetTimeLastTouchDown _returnvalue)
        (Default|PullTrigger _weapon))))
  (:Released
    (Default|ReleaseTrigger _weapon)))

(event Input|AxisEvents|InputAxisMoveUp
  (params (AxisValue :type Float%20%28single-precision%29))
  ;[1 1 1] Movement
  (Pawn|Input|AddMovementInput "1.000000, 0, 0" AxisValue false))

(event Input|AxisEvents|InputAxisMoveRight
  (params (AxisValue :type Float%20%28single-precision%29))
  ;[1 1 1] Movement
  (Pawn|Input|AddMovementInput "0.000000,1.000000, 0" AxisValue false))

(fn ConstructionScript)

(fn RelativetoCenter
  (params (x1 :type Float%20%28single-precision%29) (y1 :type Float%20%28single-precision%29) (playerController :type Player%20Controller%20Object%20Reference))
  (bind (_sizex _sizey) (HUD|GetViewportSize playerController))
  (bind _returnvalue (/ _sizey 2))
  (bind _returnvalue_2 (/ _sizex 2))
  (bind _returnvalue_3 (Math|Conversions|ToFloat(Integer) _returnvalue_2))
  (bind _returnvalue_4 (Math|Conversions|ToFloat(Integer) _returnvalue))
  (bind _returnvalue_5 (- y1 _returnvalue_4))
  (bind _returnvalue_6 (- x1 _returnvalue_3))
  (return _returnvalue_6 _returnvalue_5 (Class|KismetMathLibrary|Hypotenuse _returnvalue_6 _returnvalue_5)))