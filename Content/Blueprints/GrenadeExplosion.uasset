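; GrenadeExplosion is a grenade blast actor that spreads an expanding shockwave and damages what it overlaps.
; Each tick it widens ShockWaveMesh in X and Y by RateOfSpread, keeping its height, and destroys itself past a size limit.
; Overlapping actors that implement IDamageable and lack the Friendly tag receive Damage through the AffectHealthMessage interface call.
; The growth is per frame, without delta-time scaling, so spread speed depends on frame rate.
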(event EventBeginPlay)

(event Collision|EventActorBeginOverlap
  (params (OtherActor :type Actor%20Object%20Reference))
  (if (Utilities|DoesObjectImplementInterface OtherActor "/Game/Blueprints/iDamageable.iDamageable_C")
    (if (not (Actor|ActorHasTag OtherActor "Friendly"))
      (Class|IDamageable|AffectHealth(Message) OtherActor (Variables|Default|GetDamage)))))

(event EventTick
  (params (DeltaSeconds :type Float%20%28single-precision%29))
  (bind _rateofspread (Variables|Default|GetRateOfSpread))
  (bind _shockwavemesh (Variables|Default|GetShockWaveMesh))
  (bind _returnvalue (Transformation|GetWorldScale _shockwavemesh))
  (bind _returnvalue_2 (+ (.x _returnvalue) _rateofspread))
  (Transformation|SetWorldScale3D _shockwavemesh (Math|Vector|MakeVector _returnvalue_2 _returnvalue_2 (.z _returnvalue)))
  (if (> _returnvalue_2 17.0)
    (Actor|DestroyActor)))

(fn ConstructionScript)